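; Elevator Blueprint that moves a wall mesh when the demo character enters its trigger box with enough collected "reloj" items.
; On overlap, it compares the character's Numreloj to MaxReloj and plays a timeline that lerps SMWall3's relative location from the origin to VALORFINAL.
; Leaving the box reverses the timeline, returning the platform to its start.
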(event `self.Box.OnComponentBeginOverlap`
  (params (OverlappedComponent :type "PrimitiveComponent Object Reference") (OtherActor :type "Actor Object Reference") (OtherComp :type "PrimitiveComponent Object Reference") (OtherBodyIndex :type Integer) (bFromSweep :type Boolean) (SweepResult :type "HitResult Structure (by ref)"))
  (bind _asbp_demo_character (cast `/Game/NIVELNIVEL/NIVEL1/NIVEL1/DemoContent/Blueprints/BP_DemoCharacter` OtherActor))
  (if (>= (`/Game/NIVELNIVEL/NIVEL1/NIVEL1/DemoContent/Blueprints/BP_DemoCharacter.numreloj` _asbp_demo_character) (`self.max reloj `))
    (bind (_direction _newtrack_0) (`Timeline|Timeline` :!label _label)
      (:`Update`
        (`SceneComponent.K2_SetRelativeLocation` (`self.SM_wall3`) (`KismetMathLibrary.VLerp` (0.0 0.0 0.0) (`self.VALORFINAL`) _newtrack_0) false false)))))

(event `self.Box.OnComponentEndOverlap`
  (params (OverlappedComponent :type "PrimitiveComponent Object Reference") (OtherActor :type "Actor Object Reference") (OtherComp :type "PrimitiveComponent Object Reference") (OtherBodyIndex :type Integer))
  (cast `/Game/NIVELNIVEL/NIVEL1/NIVEL1/DemoContent/Blueprints/BP_DemoCharacter` OtherActor)
  (goto _label :!via `Reverse`))

(fn `UserConstructionScript`)