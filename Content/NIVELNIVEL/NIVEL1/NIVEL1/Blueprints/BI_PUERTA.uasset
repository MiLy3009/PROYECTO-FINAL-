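; Door Blueprint that swings a cage door open once the player has collected enough objects.
; Each collection event increments a counter, and on reaching the maximum a DoOnce triggers the open event.
; The open event plays a timeline that interpolates the cage door mesh's relative yaw to swing it open.
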(event `open puerta`
  (bind (_direction _door_rotate) (`Timeline|open puerta anim`)
    (:`Update`
      (`SceneComponent.K2_SetRelativeRotation` (`self.SM_CageDoor`) (`KismetMathLibrary.MakeRotator` 0.0 0.0 (`KismetMathLibrary.Lerp` 0.0 120.0 _door_rotate)) false false))))

(event `coleccionpuerta`
  (`/Engine/EditorBlueprintResources/StandardMacros.IncrementInt` (`self.objetosrecogidos`)
    (:`  `
      (if (>= (`self.objetosrecogidos`) (`self.maxobjetos`))
        (`/Engine/EditorBlueprintResources/StandardMacros.DoOnce` false
          (:`Completed`
            (`self.open puerta`)))))))

(fn `UserConstructionScript`)